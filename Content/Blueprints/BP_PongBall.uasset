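; BP_PongBall is the physics-driven ball for a Pong game, bouncing by rewriting its linear velocity on overlap.
; Player and enemy paddles reverse its Y velocity, pass on their own X velocity and recolor it for that side, while side walls reverse X.
; Any other overlap destroys it with a point-score particle effect, and the Destroyed event spawns a replacement at the starting position.
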(event Collision|EventActorBeginOverlap
  (params (OtherActor :type Actor%20Object%20Reference))
  (bind _asbp_pong_character (Utilities|Casting|CastToBP_PongCharacter OtherActor)
    (:then
      (bind _returnvalue (Physics|GetPhysicsLinearVelocity (Variables|Default|GetStaticMesh) "None"))
      (bind _returnvalue_2 (Physics|GetPhysicsLinearVelocity (Variables|/Game/Blueprints/Player/BP_PongCharacter.BP_PongCharacter_C|GetStaticMesh _asbp_pong_character) "None"))
      (Physics|SetPhysicsLinearVelocity (Variables|Default|GetStaticMesh) (Math|Vector|MakeVector (.X (Math|Vector|BreakVector _returnvalue_2)) (* (.Y (Math|Vector|BreakVector _returnvalue)) -1.0) (.Z (Math|Vector|BreakVector _returnvalue))) false "None")
      (Rendering|Material|SetMaterial (Variables|Default|GetStaticMesh) 0 "/Game/Materials/PlayerBallMat.PlayerBallMat"))
    (:CastFailed
      (bind _asbp_enemy_character (Utilities|Casting|CastToBP_EnemyCharacter OtherActor)
        (:then
          (bind _returnvalue_3 (Physics|GetPhysicsLinearVelocity (Variables|Default|GetStaticMesh) "None"))
          (bind _returnvalue_4 (Physics|GetPhysicsLinearVelocity (Variables|/Game/Blueprints/Player/BP_EnemyCharacter.BP_EnemyCharacter_C|GetStaticMesh _asbp_enemy_character) "None"))
          (Physics|SetPhysicsLinearVelocity (Variables|Default|GetStaticMesh) (Math|Vector|MakeVector (.X (Math|Vector|BreakVector _returnvalue_4)) (* (.Y (Math|Vector|BreakVector _returnvalue_3)) -1.0) 0.0) false "None")
          (Rendering|Material|SetMaterial (Variables|Default|GetStaticMesh) 0 "/Game/Materials/EnemyBallMat.EnemyBallMat"))
        (:CastFailed
          (Utilities|Casting|CastToBP_SideWall OtherActor
            (:then
              (bind _returnvalue_5 (Physics|GetPhysicsLinearVelocity (Variables|Default|GetStaticMesh) "None"))
              (Physics|SetPhysicsLinearVelocity (Variables|Default|GetStaticMesh) (Math|Vector|MakeVector (* (.X (Math|Vector|BreakVector _returnvalue_5)) -1.0) (.Y (Math|Vector|BreakVector _returnvalue_5)) (.Z (Math|Vector|BreakVector _returnvalue_5))) false "None"))
            (:CastFailed
              (Variables|Default|SetActorDestroyed true)
              (Actor|DestroyActor)
              (Effects|SpawnEmitteratLocation "/Game/ParticleSystem/PS_PointScore.PS_PointScore" (Transformation|GetActorLocation)))))))))

(event EventDestroyed
  (if (Variables|Default|GetActorDestroyed)
    (Game|SpawnActorfromClass "BP_PongBall_C" (Variables|Default|GetStartingPos) "Undefined" 0 0)
    (bind _output_get (Variables|Default|SetActorDestroyed false))
    (Variables|Default|SetGameStart _output_get)))

(fn ConstructionScript)