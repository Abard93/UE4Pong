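; BP_EnemyCharacter is the AI opponent paddle in a Pong-style game, tracking the ball along the X axis.
; Each Tick it finds every BP_PongBall and applies a physics force to its StaticMesh toward the ball's X position, using the clamped distance scaled by MaxSpeed.
; When it passes the X limits on either side, it snaps just inside and zeroes its velocity instead of applying force.
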(event EventTick
  (params (DeltaSeconds :type Float%20%28single-precision%29))
  (bind _returnvalue (Transformation|GetActorLocation))
  (bind _returnvalue_2 (Transformation|GetActorLocation))
  (bind _staticmesh (Variables|Default|GetStaticMesh))
  (bind (_x _y _z) (Math|Vector|BreakVector _returnvalue))
  (bind (_x_2 _y_2 _z_2) (Math|Vector|BreakVector _returnvalue_2))
  (bind _outactors (Actor|GetAllActorsOfClass "/Game/Blueprints/BP_PongBall.BP_PongBall_C"))
  (for _array_element _outactors
    (bind _asbp_pong_ball (Utilities|Casting|CastToBP_PongBall _array_element))
    (if (> (.X (Math|Vector|BreakVector (Transformation|GetActorLocation))) 8.1e+02)
      (Transformation|SetActorLocation (Math|Vector|MakeVector 809.0 _y_2 _z_2) false false)
      (Physics|SetPhysicsLinearVelocity _staticmesh "0, 0, 0" false "None")
      (elif (< (.X (Math|Vector|BreakVector (Transformation|GetActorLocation))) -8.1e+02)
        (Transformation|SetActorLocation (Math|Vector|MakeVector -809.0 _y _z) false false)
        (Physics|SetPhysicsLinearVelocity _staticmesh "0, 0, 0" false "None")
        (else
          (Physics|AddForce (Variables|Default|GetStaticMesh) (* (Math|Vector|MakeVector (Math|Float|Clamp(Float) (- (.X (Math|Vector|BreakVector (Transformation|GetActorLocation _asbp_pong_ball))) (.X (Math|Vector|BreakVector (Transformation|GetActorLocation)))) -1e+01 1e+01) 0.0 0.0) (Variables|Default|GetMax_speed)) "None" false))))))

(fn ConstructionScript)