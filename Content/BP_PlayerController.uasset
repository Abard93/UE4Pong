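; Player controller for a Pong game that moves Player 1's paddle and launches the ball.
; On BeginPlay it caches the pawn as a BP_PongCharacter.
; Each Tick it snaps the paddle back inside fixed X limits, otherwise pushes its mesh with a force from the Player1MoveUp axis scaled by MaxSpeed.
; The RespawnBall input records each unstarted ball's start transform, gives it Y velocity and flags it started.
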(event EventBeginPlay
  ;[1 1 1] Set Player 1
  (bind _asbp_pong_character (Utilities|Casting|CastToBP_PongCharacter (Game|Player|GetPlayerPawn 0)))
  (Variables|Default|SetPlayer1 _asbp_pong_character))

(event EventTick
  (params (DeltaSeconds :type Float%20%28single-precision%29))
  (bind _player1 (Variables|Default|GetPlayer1))
  (bind _returnvalue (Transformation|GetActorLocation _player1))
  (bind _returnvalue_2 (Transformation|GetActorLocation _player1))
  (bind (_x _y _z) (Math|Vector|BreakVector _returnvalue))
  (bind (_x_2 _y_2 _z_2) (Math|Vector|BreakVector _returnvalue_2))
  ;[1 1 1] Player 1 movement
  (if (> (.X (Math|Vector|BreakVector (Transformation|GetActorLocation _player1))) 8e+02)
    (Transformation|SetActorLocation _player1 (Math|Vector|MakeVector 799.0 _y_2 _z_2) false false)
    (elif (< (.X (Math|Vector|BreakVector (Transformation|GetActorLocation _player1))) -8e+02)
      (Transformation|SetActorLocation _player1 (Math|Vector|MakeVector -799.0 _y _z) false false)
      (else
        (Physics|AddForce (Variables|/Game/Blueprints/Player/BP_PongCharacter.BP_PongCharacter_C|GetStaticMesh _player1) (Math|Vector|MakeVector (* (Input|AxisValues|GetPlayer1MoveUp) (Variables|/Game/Blueprints/Player/BP_PongCharacter.BP_PongCharacter_C|GetMax_speed _player1)) 0.0 0.0) "None" false)))))

(event Input|ActionEvents|InputActionRespawnBall
  (params (Key :type Key%20Structure))
  ;[1 1 1] Start Game
  (:Pressed
    (bind _outactors (Actor|GetAllActorsOfClass "/Game/Blueprints/BP_PongBall.BP_PongBall_C"))
    (for _array_element _outactors
      (if (not (Variables|/Game/Blueprints/BP_PongBall.BP_PongBall_C|GetGameStart _array_element))
        (Variables|/Game/Blueprints/BP_PongBall.BP_PongBall_C|SetStartingPos _array_element (Transformation|GetActorTransform _array_element))
        (Physics|SetPhysicsLinearVelocity (Variables|/Game/Blueprints/BP_PongBall.BP_PongBall_C|GetStaticMesh _array_element) (Math|Vector|MakeVector 0.0 (Variables|/Game/Blueprints/BP_PongBall.BP_PongBall_C|GetStartingSpeed _array_element) 0.0) false "None")
        (Variables|/Game/Blueprints/BP_PongBall.BP_PongBall_C|SetGameStart _array_element true)))))

(fn ConstructionScript)